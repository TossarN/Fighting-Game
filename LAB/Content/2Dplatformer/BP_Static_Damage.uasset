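; BP_Static_Damage is a 2D platformer hazard that damages actors touching its ObjectSprite, limited to the player character unless CanDamageAllActors is set.
; Begin overlap sets a flag and sends DamageAmount and the hit normal through the ActorDamagedByObjectMessage interface call.
; Tick repeats that call every frame, reusing the last begin-overlap's actor and normal, until an eligible end overlap clears the single shared flag.
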(event `self.ObjectSprite.OnComponentBeginOverlap`
  (params (OverlappedComponent :type "PrimitiveComponent Object Reference") (OtherActor :type "Actor Object Reference") (OtherComp :type "PrimitiveComponent Object Reference") (OtherBodyIndex :type Integer) (bFromSweep :type Boolean) (SweepResult :type "HitResult Structure (by ref)"))
  ;[1 1 1] Start damaging actors when they overlap
  (if (`self.canDamageAllActors`)
    (set `self.isOverlappingActors` true :!label _label)
    ;;[0.1595 0.2271 1] Blueprint Interface Call
    (message `/Game/2DPlatformingKit/Blueprints/BPInterfaces/InteractionHandler.actorDamagedByObject` OtherActor (`self.DamageAmount`) (`.Normal` (`GameplayStatics.BreakHitResult` SweepResult)) :!label _label_2)
    (elif (== OtherActor (`GameplayStatics.GetPlayerCharacter` 0))
      (goto _label))))

(event `self.ReceiveTick`
  (params (DeltaSeconds :type "Float (single-precision)"))
  ;[1 1 1] Start damaging actors when they overlap
  ;;[0.1595 0.2271 1] Damages playercontinuously as well
  (if (`self.isOverlappingActors`)
    (goto _label_2)))

(event `self.ObjectSprite.OnComponentEndOverlap`
  (params (OverlappedComponent :type "PrimitiveComponent Object Reference") (OtherActor :type "Actor Object Reference") (OtherComp :type "PrimitiveComponent Object Reference") (OtherBodyIndex :type Integer))
  ;[1 1 1] Stop damaging actors when overlap ends
  (if (`self.canDamageAllActors`)
    (set `self.isOverlappingActors` false :!label _label_3)
    (elif (== OtherActor (`GameplayStatics.GetPlayerCharacter` 0))
      (goto _label_3))))

(fn `UserConstructionScript`)